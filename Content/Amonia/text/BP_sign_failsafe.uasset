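; BP_sign_failsafe is a sign actor that shows a text pop-up while its sprite is overlapped.
; On overlap, an existing inactive widget triggers BP_main's DisplayText with a fixed text enum, then joins the viewport.
; If no widget exists yet, that overlap only creates it without showing it.
; Ending the overlap removes the widget and clears its active flag.
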(event `self.sign_Sprite.OnComponentBeginOverlap`
  (params (OverlappedComponent :type "PrimitiveComponent Object Reference") (OtherActor :type "Actor Object Reference") (OtherComp :type "PrimitiveComponent Object Reference") (OtherBodyIndex :type Integer) (bFromSweep :type Boolean) (SweepResult :type "HitResult Structure (by ref)"))
  (set `self.overlap` true)
  (if (`self.overlap`)
    (if (`self.widgetActive`)
      _
      (elif (`KismetSystemLibrary.IsValid` (`self.popUp`))
        (bind _asbp_main (cast `/Game/Amonia/blueprints/BP_main` (`GameplayStatics.GetPlayerCharacter` 0)))
        (set `/Game/Amonia/blueprints/BP_main.text` "NewEnumerator2" _asbp_main)
        (`/Game/Amonia/blueprints/BP_main.DisplayText` _asbp_main)
        (`self.addWidget`)
        (else
          (bind _returnvalue (`|CreateWidget` "/Game/Amonia/Widgets/textWidget.textWidget_C" (`GameplayStatics.GetPlayerController` 0)))
          (set `self.popUp` _returnvalue))))))

(event `self.sign_Sprite.OnComponentEndOverlap`
  (params (OverlappedComponent :type "PrimitiveComponent Object Reference") (OtherActor :type "Actor Object Reference") (OtherComp :type "PrimitiveComponent Object Reference") (OtherBodyIndex :type Integer))
  (set `self.overlap` false)
  (`self.removeWidget`))

(event `addWidget`
  (`UserWidget.AddToViewport` (`self.popUp`) 0)
  (set `self.widgetActive` true))

(event `removeWidget`
  (`Widget.RemoveFromParent` (`self.popUp`))
  (set `self.widgetActive` false))

(fn `textenum`
  (returns (Value :type "/Game/Amonia/blueprints/text Enum"))
  (return (`self.Value`)))

(fn `UserConstructionScript`)