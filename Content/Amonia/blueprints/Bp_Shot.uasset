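; Bp_Shot is a shot actor with a Paper2D sprite and a sphere trigger that acts on the boar character.
; A sprite hit destroys the shot unless the other actor matches the boar reference.
; A sphere overlap with boar_char2 calls its Wereugo with the Rot variable, then destroys the shot after a short delay.
; The node setting Rot from the Arrow's world rotation is disconnected and never runs.
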(event OnComponentBeginOverlap(Sphere)
  (params (OverlappedComponent :type Primitive%20Component%20Object%20Reference) (OtherActor :type Actor%20Object%20Reference) (OtherComp :type Primitive%20Component%20Object%20Reference) (OtherBodyIndex :type Integer) (bFromSweep :type Boolean) (SweepResult :type Hit%20Result%20Structure%20%28by%20ref%29))
  (bind _asboar_char_2 (Utilities|Casting|CastToboar_char2 OtherActor))
  (Default|Wereugo _asboar_char_2 (stale _output_get))
  (Utilities|FlowControl|Delay 0.1)
  (Actor|DestroyActor))

(event OnComponentHit(PaperSprite)
  (params (HitComponent :type Primitive%20Component%20Object%20Reference) (OtherActor :type Actor%20Object%20Reference) (OtherComp :type Primitive%20Component%20Object%20Reference) (NormalImpulse :type Vector :default "0, 0, 0") (Hit :type Hit%20Result%20Structure%20%28by%20ref%29))
  (if (not (== OtherActor "/Game/Amonia/blueprints/enemy/Boar/boar_char2.boar_char2_C"))
    (Actor|DestroyActor)))

(event EventBeginPlay)

(event Collision|EventActorBeginOverlap
  (params (OtherActor :type Actor%20Object%20Reference)))

(event EventTick
  (params (DeltaSeconds :type Float%20%28single-precision%29)))

(fn ConstructionScript)