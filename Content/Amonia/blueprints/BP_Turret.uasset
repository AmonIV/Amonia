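; BP_Turret is a turret actor that repeatedly fires Bp_arrow projectiles until the player character disables it.
; After a short delay on BeginPlay, a looping retriggerable delay spawns an arrow at the Arrow component's transform at fixed intervals.
; Player overlap with the Box sets Destroyed, which is checked after each spawn, so a pending shot still fires before the loop ends.
; The actor itself stays in the level.
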(event `self.ReceiveBeginPlay`
  (`KismetSystemLibrary.Delay` 1.8)
  (`KismetSystemLibrary.RetriggerableDelay` 2.0 :!label _label)
  (`|SpawnActorFromClass` "/Game/Amonia/blueprints/Bp_arrow.Bp_arrow_C" (`SceneComponent.K2_GetComponentToWorld` (`self.Arrow`)) "AlwaysSpawn" "OverrideRootScale")
  (if (not (`self.destroyed`))
    (goto _label)))

(event `self.Box.OnComponentBeginOverlap`
  (params (OverlappedComponent :type "PrimitiveComponent Object Reference") (OtherActor :type "Actor Object Reference") (OtherComp :type "PrimitiveComponent Object Reference") (OtherBodyIndex :type Integer) (bFromSweep :type Boolean) (SweepResult :type "HitResult Structure (by ref)"))
  (if (== (`GameplayStatics.GetPlayerCharacter` 0) OtherActor)
    (set `self.destroyed` true)))

(fn `UserConstructionScript`)