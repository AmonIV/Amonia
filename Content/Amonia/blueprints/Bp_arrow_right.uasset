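; Right-arrow projectile actor with a Paper2D sprite that damages the player on impact.
; When the sprite hits the player, it sets the BP_main character's Facing to -1, passes its Damage to that character's DamageSystem and destroys itself.
; It also destroys itself on hitting anything else, or 1.5 seconds after BeginPlay.
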(event `self.ReceiveBeginPlay`
  (`KismetSystemLibrary.Delay` 1.5)
  (`self.K2_DestroyActor`))

(event `self.PaperSprite.OnComponentHit`
  (params (HitComponent :type "PrimitiveComponent Object Reference") (OtherActor :type "Actor Object Reference") (OtherComp :type "PrimitiveComponent Object Reference") (NormalImpulse :type "Vector Structure") (Hit :type "HitResult Structure (by ref)"))
  (bind _returnvalue (`GameplayStatics.GetPlayerCharacter` 0))
  (if (== _returnvalue OtherActor)
    (bind _asbp_main (cast `/Game/Amonia/blueprints/BP_main` _returnvalue))
    (set `/Game/Amonia/blueprints/BP_main.Facing` -1 _asbp_main)
    (bind _asbp_main_2 (cast `/Game/Amonia/blueprints/BP_main` (`GameplayStatics.GetPlayerCharacter` 0)))
    (`/Game/Amonia/blueprints/BP_main.DamageSystem` _asbp_main_2 (`self.Damage`))
    (`self.K2_DestroyActor`)
    (else
      (`self.K2_DestroyActor`))))

(event `self.PaperSprite.OnComponentBeginOverlap`
  (params (OverlappedComponent :type "PrimitiveComponent Object Reference") (OtherActor :type "Actor Object Reference") (OtherComp :type "PrimitiveComponent Object Reference") (OtherBodyIndex :type Integer) (bFromSweep :type Boolean) (SweepResult :type "HitResult Structure (by ref)")))

(fn `UserConstructionScript`)