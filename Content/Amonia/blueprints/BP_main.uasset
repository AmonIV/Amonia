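; Player character for Amonia's 2D side-scroller, handling movement, sprint, jumping with a boots-gated double jump, and rock throwing.
; A Stance variable drives flipbook swaps, set by input, landing and damage events that apply knockback, death and gas damage.
; Custom events provide impulse-based pad and wall bounces plus timed invincibility.
; It also creates the HUD, menu, pause, death and level-end widgets, selects tutorial and dialogue text, and handles level restart.
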(event `DamageSystem`
  (params (Damage :type "Float (double-precision)"))
  ;[1 1 1] damage system
  (if (not (`self.Invincible`))
    (set `self.Is_Hit` true)
    (`self.DisableInput` (`GameplayStatics.GetPlayerController` 0))
    (`MovementComponent.StopMovementImmediately` (`self.CharacterMovement`))
    (bind _output_get (set `self.Health_current` (- (`self.Health_current`) Damage)))
    (if (<= _output_get 0.0)
      (set `self.Stance` "NewEnumerator5" :!label _label)
      (`self.DisableInput` (`GameplayStatics.GetPlayerController` 0))
      (`KismetSystemLibrary.Delay` 1.0)
      (`self.PlayerDead`)
      (else
        (set `self.Stance` "NewEnumerator4")
        (`CharacterMovementComponent.AddImpulse` (`self.CharacterMovement`) (`KismetMathLibrary.MakeVector` (* (`self.Facing`) (`self.Knockback`)) 0.0 400.0) true)))))

(event `Stage1`
  (bind _returnvalue (`GameplayStatics.GetPlayerController` 0))
  ;[1 1 1] stage 1
  (bind _returnvalue_2 (`|CreateWidget` "/Game/Amonia/Widgets/Level_select1.Level_select1_C" _returnvalue))
  (`UserWidget.AddToViewport` _returnvalue_2 0)
  (set `PlayerController.bShowMouseCursor` true _returnvalue)
  (`WidgetBlueprintLibrary.SetInputMode_UIOnlyEx` _returnvalue _returnvalue_2))

(event `Key|Escape`
  (params (Key :type "Key Structure" :default "AnyKey"))
  (bind _pause (`self.Pause`))
  ;[1 1 1] Game Pause
  (:`Pressed`
    (`/Engine/EditorBlueprintResources/StandardMacros.IsValid` _pause
      (:`Is Valid`
        _)
      (:`Is Not Valid`
        (bind _returnvalue (`|CreateWidget` "/Game/Amonia/Widgets/PauseGame.PauseGame_C"))
        (bind _output_get (set `self.Pause` _returnvalue))))
    (`WidgetBlueprintLibrary.SetInputMode_UIOnlyEx` (`GameplayStatics.GetPlayerController` 0) _pause)
    (`UserWidget.AddToViewport` _output_get 0)
    (set `PlayerController.bShowMouseCursor` true (`GameplayStatics.GetPlayerController` 0))
    (`GameplayStatics.SetGamePaused` true)
    (set `self.Resetable` false)))

(event `Key|F`
  (params (Key :type "Key Structure" :default "AnyKey"))
  ;[1 1 1] Attempt to Talk
  (:`Pressed`
    (set `self.AttemptTalk` true)
    (`KismetSystemLibrary.Delay` 0.5)
    (set `self.AttemptTalk` false)))

(event `Gas_Damage`
  (params (damage :type "Float (double-precision)"))
  ;[1 1 1] damage system
  (if (not (`self.Invincible`))
    (bind _output_get (set `self.Health_current` (- (`self.Health_current`) damage)))
    (if (<= _output_get 0.0)
      (goto _label))))

(event `SignTransfer`
  ;[1 1 1] tutorial start
  (`CharacterMovementComponent.AddImpulse` (`self.CharacterMovement`) (200.0 0.0 100.0) true))

(event `PlayerDead`
  (bind _returnvalue (`GameplayStatics.GetPlayerController` 0))
  ;[1 1 1] Player Dead
  (`self.DisableInput` (`GameplayStatics.GetPlayerController` 0))
  (bind _returnvalue_2 (`|CreateWidget` "/Game/Amonia/Widgets/DeathScreen.DeathScreen_C" _returnvalue))
  (`UserWidget.AddToViewport` _returnvalue_2 0)
  (set `PlayerController.bShowMouseCursor` true _returnvalue)
  (`WidgetBlueprintLibrary.SetInputMode_UIOnlyEx` _returnvalue _returnvalue_2)
  (set `self.Resetable` false))

(event `InputAction|Jump`
  (params (Key :type "Key Structure" :default "AnyKey"))
  ;[1 1 1] Handle Jump
  (:`Pressed`
    (`self.Jump` :!label _label_2)
    (set `self.Stance` "NewEnumerator2"))
  (:`Released`
    (`self.StopJumping` :!label _label_3)))

(event `InputTouch`
  (params (Location :type "Vector Structure") (FingerIndex :type "ETouchIndex Enum"))
  ;[1 1 1] Handle Jump
  (:`Pressed`
    (goto _label_2))
  (:`Released`
    (goto _label_3)))

(event `UpdateAnimation`
  ;[1 1 1] Handle Animation
  (switch `/Game/Amonia/blueprints/Char_state` (`self.Stance`)
    (:`NewEnumerator0`
      (`PaperFlipbookComponent.SetFlipbook` (`self.Sprite`) (select `bool` (> (`KismetMathLibrary.VSize` (`self.GetVelocity`)) 0.0) :`false` "/Game/Amonia/Sprites/character/A_idle.A_idle" :`true` "/Game/Amonia/Sprites/character/A_walk.A_walk" :!type "PaperFlipbook Object Reference")))
    (:`NewEnumerator2`
      (`PaperFlipbookComponent.SetFlipbook` (`self.Sprite`) "/Game/Amonia/Sprites/character/A_jump.A_jump"))
    (:`NewEnumerator4`
      (`PaperFlipbookComponent.SetFlipbook` (`self.Sprite`) "/Game/Amonia/Sprites/character/A_hit.A_hit"))
    (:`NewEnumerator5`
      (`PaperFlipbookComponent.SetFlipbook` (`self.Sprite`) "/Game/Amonia/Sprites/character/A_Dead.A_Dead"))
    (:`NewEnumerator6`
      (`PaperFlipbookComponent.SetFlipbook` (`self.Sprite`) "/Game/Amonia/Sprites/character/A_sit.A_sit"))
    (:`NewEnumerator7`
      (`PaperFlipbookComponent.SetFlipbook` (`self.Sprite`) "/Game/Amonia/Sprites/character/A_GroundThrow.A_GroundThrow"))))

(event `self.ReceiveTick`
  (params (DeltaSeconds :type "Float (single-precision)"))
  ;[1 1 1] Handle Animation
  (`self.UpdateAnimation`))

(event `LevelEnd`
  (bind _returnvalue (`GameplayStatics.GetPlayerController` 0))
  ;[1 1 1] End Level
  (bind _returnvalue_2 (`|CreateWidget` "/Game/Amonia/Widgets/EndOfLevel.EndOfLevel_C" _returnvalue))
  (`UserWidget.AddToViewport` _returnvalue_2 0)
  (set `PlayerController.bShowMouseCursor` true _returnvalue)
  (`WidgetBlueprintLibrary.SetInputMode_UIOnlyEx` _returnvalue _returnvalue_2)
  (set `self.Resetable` false))

(event `tutorial start`
  (bind _returnvalue (`GameplayStatics.GetPlayerController` 0))
  ;[1 1 1] tutorial start
  (bind _returnvalue_2 (`|CreateWidget` "/Game/Amonia/Widgets/MainMenu.MainMenu_C" (`GameplayStatics.GetPlayerController` 0)))
  (`UserWidget.AddToViewport` _returnvalue_2 0)
  (set `PlayerController.bShowMouseCursor` true _returnvalue)
  (`WidgetBlueprintLibrary.SetInputMode_UIOnlyEx` _returnvalue _returnvalue_2)
  (set `self.Resetable` false))

(event `self.ReceiveBeginPlay`
  ;[1 0.07087 0.8099] Start
  (`|ExecutionSequence`
    (:`then_0`
      (`ActorComponent.SetIsReplicated` (`self.Sprite`) true))
    (:`then_1`
      (bind _returnvalue (`|CreateWidget` "/Game/Amonia/Widgets/Hud.Hud_C" (`GameplayStatics.GetPlayerController` 0)))
      (bind _output_get (set `self.Health_bar` _returnvalue))
      (`UserWidget.AddToViewport` _output_get 0))))

(event `DisplayText`
  ;[1 1 1] Text To Screen
  (switch `/Game/Amonia/blueprints/text` (`self.text`)
    (:`NewEnumerator1`
      (set `self.CurrentString` "Hello player and welcome to The land of Amonia. Use A/D to move left and right. Use W or Space to jump."))
    (:`NewEnumerator2`
      (set `self.CurrentString` "There are spikes in front of you! Try to jump over them."))
    (:`NewEnumerator3`
      (set `self.CurrentString` "These are skybushes. They are charged with magical eneregy that allows them to set roots in mid air. You can jump on them to go between islands."))
    (:`NewEnumerator4`
      (set `self.CurrentString` "Seems like there is an arrow turret standing in your way. Dodge the arrows and get to the turret to disable it."))
    (:`NewEnumerator5`
      (set `self.CurrentString` "Well that wasn't too hard! The next part is a bit more difficult. Try to disable the turret!"))
    (:`NewEnumerator6`
      (set `self.CurrentString` "You finished the tutorial! Walk forward to finish."))
    (:`NewEnumerator7`
      (set `self.CurrentString` "During your journey you will meet other characters. One of them owns this house. Go near them and press 'f' to talk."))
    (:`NewEnumerator8`
      (set `self.CurrentString` "Secret knowledge : Press the left mouse button to throw rocks."))
    (:`NewEnumerator10`
      (set `self.CurrentString` "You found an easter egg!"))
    (:`NewEnumerator9`
      (set `self.CurrentString` "This seems to be the owner of this house..."))
    (:`NewEnumerator11`
      (set `self.CurrentString` "House owner : Hello There!"))
    (:`NewEnumerator12`
      (set `self.CurrentString` "House owner : If you get hurt be sure to eat some berries from a berry bush. They will heal you."))
    (:`NewEnumerator13`
      (set `self.CurrentString` "House owner : There are some in front of my house if you need them."))
    (:`NewEnumerator14`
      (set `self.CurrentString` "You : Thank you"))
    (:`NewEnumerator16`
      (set `self.CurrentString` "*Before you stands a man in a magnificent hat*"))))

(event `Stage select`
  (bind _returnvalue (`GameplayStatics.GetPlayerController` 0))
  ;[1 1 1] Stage select
  (bind _returnvalue_2 (`|CreateWidget` "/Game/Amonia/Widgets/Stage_select.Stage_select_C" _returnvalue))
  (`UserWidget.AddToViewport` _returnvalue_2 0)
  (set `PlayerController.bShowMouseCursor` true _returnvalue)
  (`WidgetBlueprintLibrary.SetInputMode_UIOnlyEx` _returnvalue _returnvalue_2))

(event `InputAction|Sprint`
  (params (Key :type "Key Structure" :default "AnyKey"))
  ;[1 1 1] Sprint
  (:`Pressed`
    (set `self.Movementmultiplier` 0.75))
  (:`Released`
    (set `self.Movementmultiplier` 0.5)))

(event `Invincibility`
  ;[1 1 1] invincibility
  (set `self.Invincible` true)
  (`KismetSystemLibrary.Delay` 0.5)
  (set `self.Invincible` false)
  (set `self.Is_Hit` false))

(event `self.OnLanded`
  (params (Hit :type "HitResult Structure (by ref)"))
  ;[1 1 1] landing
  (if (`self.Is_Hit`)
    (if (<= (`self.Health_current`) 0.0)
      (set `self.Stance` "NewEnumerator5")
      (`self.DisableInput` (`GameplayStatics.GetPlayerController` 0))
      (`self.UpdateAnimation`)
      (else
        (set `self.Stance` "NewEnumerator6")
        (`self.UpdateAnimation`)
        (`KismetSystemLibrary.Delay` 0.5)
        (set `self.Is_Hit` false)
        (set `self.Stance` "NewEnumerator0")
        (`self.UpdateAnimation`)
        (`self.EnableInput` (`GameplayStatics.GetPlayerController` 0))))
    (else
      (set `self.Stance` "NewEnumerator0")
      (set `self.djump` 0)
      (`self.UpdateAnimation`))))

(event `InputAxis|MoveRight`
  (params (AxisValue :type "Float (single-precision)"))
  ;[1 1 1] Handle movement
  (if (not (`self.talking`))
    (if (> AxisValue 0.0)
      (set `self.bisMovingRight` true)
      (elif (< AxisValue 0.0)
        (set `self.bisMovingRight` false)))
    (`self.AddMovementInput` (1.0 0.0 0.0) (* AxisValue (`self.Movementmultiplier`)))
    ;[1 1 1] Tick - Updates animation
    (`self.UpdateAnimation`)
    (`/Engine/EditorBlueprintResources/StandardMacros.CompareFloat` AxisValue
      (:`>`
        (`Controller.SetControlRotation` (`self.GetController`) (`KismetMathLibrary.MakeRotator` 0.0 0.0 0.0) :!label _label_4)
        (set `self.Facing` 1))
      (:`==`
        (if (`self.bisMovingRight`)
          (goto _label_4)
          (else
            (`Controller.SetControlRotation` (`self.GetController`) (`KismetMathLibrary.MakeRotator` 0.0 0.0 180.0) :!label _label_5)
            (set `self.Facing` -1))))
      (:`<`
        (goto _label_5)))))

(event `InputAction|Shoot`
  (params (Key :type "Key Structure" :default "AnyKey"))
  (bind _returnvalue (`GameplayStatics.GetPlayerController` 0))
  ;[1 1 1] shoot
  (:`Pressed`
    (if (`self.canThrow`)
      (`self.DisableInput` _returnvalue)
      (set `self.Stance` "NewEnumerator7")
      (`self.UpdateAnimation`)
      (`KismetSystemLibrary.RetriggerableDelay` 0.2)
      (`|SpawnActorFromClass` "/Game/Amonia/blueprints/Bp_Shot.Bp_Shot_C" (`SceneComponent.K2_GetComponentToWorld` (`self.Arrow1`)) "AlwaysSpawn" "OverrideRootScale")
      (`KismetSystemLibrary.RetriggerableDelay` 0.3)
      (`self.EnableInput` _returnvalue)
      (set `self.Stance` "NewEnumerator0")
      (`self.UpdateAnimation`))))

(event `Bounce_pad`
  (bind _charactermovement (`self.CharacterMovement`))
  (bind _fall_velocity (`self.fall_velocity`))
  ;[1 1 1] Bpad
  (`MovementComponent.StopMovementImmediately` _charactermovement)
  (`CharacterMovementComponent.AddImpulse` _charactermovement (`KismetMathLibrary.MakeVector` (`self.Side_velocity`) 0.0 _fall_velocity) true)
  (`KismetSystemLibrary.PrintString` (`KismetStringLibrary.Conv_DoubleToString` _fall_velocity)))

(event `InputAction|Jump`
  (params (Key :type "Key Structure" :default "AnyKey"))
  ;[1 1 1] double jump
  (:`Pressed`
    (if (`self.Has_boots`)
      (if (`|EnumEquality` (`self.Stance`) "NewEnumerator2")
        (if (< (`self.djump`) 1)
          (set `self.djump` (+ (`self.djump`) 1))
          (`self.vel_calc`)
          (`self.Continue_jump`))))))

(event `Bounce_pad_vel`
  (bind (_velocity_x _velocity_y _velocity_z) (`KismetMathLibrary.BreakVector` (`MovementComponent.Velocity` (`self.CharacterMovement`))))
  ;[1 1 1] Bpad
  (set `self.fall_velocity` (+ (* _velocity_z -1.0) 0.0))
  (set `self.Side_velocity` _velocity_x))

(event `WallBounceRight`
  (bind _returnvalue (`GameplayStatics.GetPlayerController` 0))
  (bind _charactermovement (`self.CharacterMovement`))
  ;[1 1 1] Bounce 300
  (`self.DisableInput` _returnvalue)
  (`MovementComponent.StopMovementImmediately` _charactermovement)
  (`CharacterMovementComponent.AddImpulse` _charactermovement (300.0 0.0 300.0) true)
  (`KismetSystemLibrary.Delay` 0.2)
  (`self.EnableInput` _returnvalue))

(event `WallBounceRight400`
  (bind _returnvalue (`GameplayStatics.GetPlayerController` 0))
  (bind _charactermovement (`self.CharacterMovement`))
  ;[1 1 1] Bounce 400
  (`self.DisableInput` _returnvalue)
  (`MovementComponent.StopMovementImmediately` _charactermovement)
  (`CharacterMovementComponent.AddImpulse` _charactermovement (300.0 0.0 400.0) true)
  (`KismetSystemLibrary.Delay` 0.2)
  (`self.EnableInput` _returnvalue))

(event `Continue_jump`
  (bind _fall_velocity (`self.fall_velocity`))
  (bind _charactermovement (`self.CharacterMovement`))
  ;[1 1 1] double jump
  (`MovementComponent.StopMovementImmediately` _charactermovement)
  (`CharacterMovementComponent.AddImpulse` _charactermovement (`KismetMathLibrary.MakeVector` (`self.Side_velocity`) 0.0 _fall_velocity) true)
  (`KismetSystemLibrary.PrintString` (`KismetStringLibrary.Conv_DoubleToString` _fall_velocity)))

(event `vel_calc`
  (bind (_velocity_x _velocity_y _velocity_z) (`KismetMathLibrary.BreakVector` (`MovementComponent.Velocity` (`self.CharacterMovement`))))
  ;[1 1 1] double jump
  (bind _output_get (set `self.fall_velocity` (* _velocity_z 1.0)))
  (set `self.Side_velocity` _velocity_x)
  (if (< _output_get 0.0)
    (set `self.fall_velocity` 450.0)
    (else
      (set `self.fall_velocity` (+ (`self.fall_velocity`) 450.0)))))

(event `InputAction|Restart`
  (params (Key :type "Key Structure" :default "AnyKey"))
  ;[1 1 1] level reset
  (:`Pressed`
    (if (`self.Resetable`)
      (`GameplayStatics.OpenLevel` (`self.current_level`)))))

(event `WallBounceLeft400`
  (bind _returnvalue (`GameplayStatics.GetPlayerController` 0))
  (bind _charactermovement (`self.CharacterMovement`))
  ;[1 1 1] Bounce 400
  (`self.DisableInput` _returnvalue)
  (`MovementComponent.StopMovementImmediately` _charactermovement)
  (`CharacterMovementComponent.AddImpulse` _charactermovement (-300.0 0.0 400.0) true)
  (`KismetSystemLibrary.Delay` 0.2)
  (`self.EnableInput` _returnvalue))

(event `WallBounceLeft`
  (bind _returnvalue (`GameplayStatics.GetPlayerController` 0))
  (bind _charactermovement (`self.CharacterMovement`))
  ;[1 1 1] Bounce 300
  (`self.DisableInput` _returnvalue)
  (`MovementComponent.StopMovementImmediately` _charactermovement)
  (`CharacterMovementComponent.AddImpulse` _charactermovement (-300.0 0.0 300.0) true)
  (`KismetSystemLibrary.Delay` 0.2)
  (`self.EnableInput` _returnvalue))

(event `Custom_right`
  (bind _returnvalue (`GameplayStatics.GetPlayerController` 0))
  (bind _charactermovement (`self.CharacterMovement`))
  ;[1 1 1] custom
  (`self.DisableInput` _returnvalue)
  (`MovementComponent.StopMovementImmediately` _charactermovement)
  (`CharacterMovementComponent.AddImpulse` _charactermovement (`KismetMathLibrary.MakeVector` (`self.Bounce_right`) 0.0 (`self.Bounce_up`)) true)
  (`KismetSystemLibrary.Delay` 0.2)
  (`self.EnableInput` _returnvalue))

(event `Custom_left`
  (bind _returnvalue (`GameplayStatics.GetPlayerController` 0))
  (bind _charactermovement (`self.CharacterMovement`))
  ;[1 1 1] custom
  (`self.DisableInput` _returnvalue)
  (`MovementComponent.StopMovementImmediately` _charactermovement)
  (`CharacterMovementComponent.AddImpulse` _charactermovement (`KismetMathLibrary.MakeVector` (* (`self.Bounce_left`) -1.0) 0.0 (`self.Bounce_up`)) true)
  (`KismetSystemLibrary.Delay` 0.2)
  (`self.EnableInput` _returnvalue))

(fn `UserConstructionScript`)