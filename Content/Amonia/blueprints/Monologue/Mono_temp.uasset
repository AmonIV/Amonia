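; Temporary monologue trigger that shows a Mono_temp_widget when the player enters its Box.
; On overlap it creates the widget, sets the string and Talking flag on BP_main, and switches to UI-only input with a cursor.
; It polls the widget's Ded flag every 0.2 seconds, then removes the widget and destroys itself.
; Leaving the box also removes the widget; the AttemptTalk check gates nothing and its retry loop is disconnected.
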(event `self.Box.OnComponentBeginOverlap`
  (params (OverlappedComponent :type "PrimitiveComponent Object Reference") (OtherActor :type "Actor Object Reference") (OtherComp :type "PrimitiveComponent Object Reference") (OtherBodyIndex :type Integer) (bFromSweep :type Boolean) (SweepResult :type "HitResult Structure (by ref)"))
  (bind _returnvalue (`GameplayStatics.GetPlayerController` 0))
  (bind _returnvalue_2 (`GameplayStatics.GetPlayerCharacter` 0))
  (if (== OtherActor _returnvalue_2)
    (`|ExecutionSequence`
      (:`then_0`
        (set `self.overlap` true)
        (if (`self.overlap`)
          (if (`self.widgetActive`)
            _
            (elif (not (`KismetSystemLibrary.IsValid` (`self.mono_d`)))
              ;[1 1 1] rep
              (bind _returnvalue_3 (`|CreateWidget` "/Game/Amonia/blueprints/Monologue/Mono_temp_widget.Mono_temp_widget_C" (`GameplayStatics.GetPlayerController` 0)))
              (set `self.mono_d` _returnvalue_3)
              (bind _asbp_main (cast `/Game/Amonia/blueprints/BP_main` (`GameplayStatics.GetPlayerCharacter` 0)))
              ;[1 1 1] rep
              (set `/Game/Amonia/blueprints/BP_main.CurrentString` "ez" _asbp_main)
              (set `self.text` "NewEnumerator0")))))
      (:`then_1`
        (bind _asbp_main_2 (cast `/Game/Amonia/blueprints/BP_main` _returnvalue_2))
        (if (`/Game/Amonia/blueprints/BP_main.AttemptTalk` _asbp_main_2)
          _
          (else
            _))
        (set `self.talking` true)
        (`self.addWidget`)
        (bind _asbp_main_3 (cast `/Game/Amonia/blueprints/BP_main` (`GameplayStatics.GetPlayerCharacter` 0)))
        (set `/Game/Amonia/blueprints/BP_main.talking` true _asbp_main_3)
        (`WidgetBlueprintLibrary.SetInputMode_UIOnlyEx` _returnvalue (`self.mono_d`))
        (set `PlayerController.bShowMouseCursor` true _returnvalue)
        (if (`/Game/Amonia/blueprints/Monologue/Mono_temp_widget.ded` (`self.mono_d`)) :!label _label
          (`self.removeWidget`)
          (`self.K2_DestroyActor`)
          (else
            (`KismetSystemLibrary.Delay` 0.2)
            (goto _label)))))))

(event `self.Box.OnComponentEndOverlap`
  (params (OverlappedComponent :type "PrimitiveComponent Object Reference") (OtherActor :type "Actor Object Reference") (OtherComp :type "PrimitiveComponent Object Reference") (OtherBodyIndex :type Integer))
  (if (== OtherActor (`GameplayStatics.GetPlayerCharacter` 0))
    (set `self.overlap` false)
    (`self.removeWidget`)))

(event `addWidget`
  (`UserWidget.AddToViewport` (`self.mono_d`) 0)
  (set `self.widgetActive` true))

(event `removeWidget`
  (`Widget.RemoveFromParent` (`self.mono_d`))
  (set `self.widgetActive` false))

(fn `textenum`
  (returns (Value :type "/Game/Amonia/blueprints/text Enum"))
  (return (`self.Value`)))

(fn `UserConstructionScript`)