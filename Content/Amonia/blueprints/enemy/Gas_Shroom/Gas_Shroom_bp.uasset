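; Gas mushroom hazard that releases a short-lived damaging cloud when the player walks into its trigger Box.
; After a short delay it shows six gas sprites and sets Gas, then hides and clears them through a retriggerable delay.
; Gas_box tracks whether the player is inside, and a looped delay calls GasDamage on BP_main every second while gassed.
; Update re-evaluates that state on each gas toggle, starting damage for a player already inside.
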(event `self.Box.OnComponentBeginOverlap`
  (params (OverlappedComponent :type "PrimitiveComponent Object Reference") (OtherActor :type "Actor Object Reference") (OtherComp :type "PrimitiveComponent Object Reference") (OtherBodyIndex :type Integer) (bFromSweep :type Boolean) (SweepResult :type "HitResult Structure (by ref)"))
  (if (== OtherActor (`GameplayStatics.GetPlayerCharacter` 0))
    (`KismetSystemLibrary.Delay` 1.5)
    (`SceneComponent.SetHiddenInGame` (`self.gas_Sprite`) false false)
    (`SceneComponent.SetHiddenInGame` (`self.gas2`) false false)
    (`SceneComponent.SetHiddenInGame` (`self.gas3`) false false)
    (`SceneComponent.SetHiddenInGame` (`self.gas4`) false false)
    (`SceneComponent.SetHiddenInGame` (`self.gas5`) false false)
    (`SceneComponent.SetHiddenInGame` (`self.gas6`) false false)
    (set `self.gas` true)
    (`self.update`)
    (`KismetSystemLibrary.RetriggerableDelay` 2.0)
    (`SceneComponent.SetHiddenInGame` (`self.gas_Sprite`) true false)
    (`SceneComponent.SetHiddenInGame` (`self.gas2`) true false)
    (`SceneComponent.SetHiddenInGame` (`self.gas3`) true false)
    (`SceneComponent.SetHiddenInGame` (`self.gas4`) true false)
    (`SceneComponent.SetHiddenInGame` (`self.gas5`) true false)
    (`SceneComponent.SetHiddenInGame` (`self.gas6`) true false)
    (set `self.gas` false)
    (`self.update`)))

(event `self.gas_box.OnComponentBeginOverlap`
  (params (OverlappedComponent :type "PrimitiveComponent Object Reference") (OtherActor :type "Actor Object Reference") (OtherComp :type "PrimitiveComponent Object Reference") (OtherBodyIndex :type Integer) (bFromSweep :type Boolean) (SweepResult :type "HitResult Structure (by ref)"))
  (bind _returnvalue (`GameplayStatics.GetPlayerCharacter` 0))
  (if (== OtherActor _returnvalue)
    (set `self.in` true)
    (if (`self.gas`)
      (set `self.gassed` true)
      (if (`self.gassed`) :!label _label
        (if (`self.gas`)
          (bind _asbp_main (cast `/Game/Amonia/blueprints/BP_main` _returnvalue))
          (`/Game/Amonia/blueprints/BP_main.Gas_Damage` _asbp_main 0.1)
          (`KismetSystemLibrary.Delay` 1.0)
          (goto _label))))))

(event `force_gas`
  (goto _label))

(event `self.gas_box.OnComponentEndOverlap`
  (params (OverlappedComponent :type "PrimitiveComponent Object Reference") (OtherActor :type "Actor Object Reference") (OtherComp :type "PrimitiveComponent Object Reference") (OtherBodyIndex :type Integer))
  (if (== OtherActor (`GameplayStatics.GetPlayerCharacter` 0))
    (set `self.in` false)
    (set `self.gassed` false)))

(event `update`
  (if (`self.in`)
    (set `self.gassed` true)
    (`self.force_gas`)
    (else
      (set `self.gassed` false))))

(fn `UserConstructionScript`)