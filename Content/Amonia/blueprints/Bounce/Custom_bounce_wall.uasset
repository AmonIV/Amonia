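; Bounce wall actor with left and right trigger boxes that act only on the player's BP_main character.
; When the player overlaps a box, it zeroes that side's bounce value (BounceLeft or BounceRight) along with BounceUp on the character.
; It then calls CustomLeft or CustomRight on BP_main, leaving the actual response to the character.
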(event `self.Box_left.OnComponentBeginOverlap`
  (params (OverlappedComponent :type "PrimitiveComponent Object Reference") (OtherActor :type "Actor Object Reference") (OtherComp :type "PrimitiveComponent Object Reference") (OtherBodyIndex :type Integer) (bFromSweep :type Boolean) (SweepResult :type "HitResult Structure (by ref)"))
  (bind _returnvalue (`GameplayStatics.GetPlayerCharacter` 0))
  (bind _asbp_main (cast `/Game/Amonia/blueprints/BP_main` _returnvalue))
  (if (== OtherActor _asbp_main)
    (bind _asbp_main_2 (cast `/Game/Amonia/blueprints/BP_main` _returnvalue))
    (set `/Game/Amonia/blueprints/BP_main.Bounce_left` 0.0 _asbp_main_2)
    (set `/Game/Amonia/blueprints/BP_main.Bounce_up` 0.0 _asbp_main_2)
    (`/Game/Amonia/blueprints/BP_main.Custom_left` _asbp_main_2)))

(event `self.Box_right.OnComponentBeginOverlap`
  (params (OverlappedComponent :type "PrimitiveComponent Object Reference") (OtherActor :type "Actor Object Reference") (OtherComp :type "PrimitiveComponent Object Reference") (OtherBodyIndex :type Integer) (bFromSweep :type Boolean) (SweepResult :type "HitResult Structure (by ref)"))
  (bind _returnvalue (`GameplayStatics.GetPlayerCharacter` 0))
  (bind _asbp_main (cast `/Game/Amonia/blueprints/BP_main` _returnvalue))
  (if (== _asbp_main OtherActor)
    (bind _asbp_main_2 (cast `/Game/Amonia/blueprints/BP_main` _returnvalue))
    (set `/Game/Amonia/blueprints/BP_main.Bounce_right` 0.0 _asbp_main_2)
    (set `/Game/Amonia/blueprints/BP_main.Bounce_up` 0.0 _asbp_main_2)
    (`/Game/Amonia/blueprints/BP_main.Custom_right` _asbp_main_2)))

(fn `UserConstructionScript`)